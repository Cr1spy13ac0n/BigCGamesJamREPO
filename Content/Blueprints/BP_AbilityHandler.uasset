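; BP_AbilityHandler runs the cancer-treatment abilities, destroying cell actors and counting the kills.
; Chemotherapy gives every cancer cell a high random chance of destruction.
; Radiotherapy lights the BP_Camera spotlight as a prepped state; RadioFinish switches it off and sphere-traces from it, destroying everything hit and tallying cancer versus friendly losses.
; A small score function adds radiotherapy kills to an inherited score, while the health function is empty.
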(event Custom|Chemotherapy
  (Variables|Default|SetFriendly%20Destroyed 0)
  (Variables|Default|SetCancer%20Destroyed 0)
  (bind _outactors (Actor|GetAllActorsOfClass "/Game/Blueprints/Bp_Cell_Child_CancerCell.Bp_Cell_Child_CancerCell_C"))
  (for _array_element _outactors
    (if (not (>= (Math|Random|RandomFloatinRange 0.0 1.0) 0.95))
      (bind _output_get (Variables|Default|SetCancer%20Destroyed (+ (Variables|Default|GetCancer%20Destroyed) 1)))
      (Development|PrintString (Utilities|String|ToString(Integer) _output_get))
      (Actor|DestroyActor _array_element))))

(event Custom|Radiotherapy
  (bind _returnvalue (Actor|GetActorOfClass "/Game/Blueprints/BP_Camera.BP_Camera_C"))
  (Rendering|Components|Light|SetIntensity (Variables|/Game/Blueprints/BP_Camera.BP_Camera_C|GetSpotLight _returnvalue) 5.0)
  (Variables|Default|SetRadioTherapyPrepped true))

(event Custom|RadioFinish
  (bind _returnvalue (Actor|GetActorOfClass "/Game/Blueprints/BP_Camera.BP_Camera_C"))
  (Variables|Default|SetCamera%20Obj%20Ref _returnvalue)
  (Variables|Default|SetFriendly%20Destroyed 0)
  (Variables|Default|SetCancer%20Destroyed 0)
  (Rendering|Components|Light|SetIntensity (Variables|/Game/Blueprints/BP_Camera.BP_Camera_C|GetSpotLight (Variables|Default|GetCamera%20Obj%20Ref)) 0.0)
  (Variables|Default|SetRadioTherapyPrepped false)
  (bind _outhits (Collision|MultiSphereTraceByChannel (Transformation|GetWorldLocation (Variables|/Game/Blueprints/BP_Camera.BP_Camera_C|GetSpotLight _returnvalue)) (+ (Transformation|GetWorldLocation (Variables|/Game/Blueprints/BP_Camera.BP_Camera_C|GetSpotLight _returnvalue)) (* (Math|Vector|MakeVector (.x (Math|Vector|GetUpVector (Variables|/Game/Blueprints/BP_Camera.BP_Camera_C|GetSpotLight _returnvalue))) (.y (Math|Vector|GetUpVector (Variables|/Game/Blueprints/BP_Camera.BP_Camera_C|GetSpotLight _returnvalue))) (+ (.z (Math|Vector|GetUpVector (Variables|/Game/Blueprints/BP_Camera.BP_Camera_C|GetSpotLight _returnvalue))) 9e+01)) -1e+05)) 4.1e+02 "TraceTypeQuery3" false 0 "Persistent"))
  (for _array_element _outhits
    (if (== (Utilities|GetClass (.hitactor _array_element)) "/Game/Blueprints/Bp_Cell_Child_CancerCell.Bp_Cell_Child_CancerCell_C")
      (Variables|Default|SetCancer%20Destroyed (+ (Variables|Default|GetCancer%20Destroyed) 1))
      (Actor|DestroyActor (.hitactor _array_element))
      (else
        (Variables|Default|SetFriendly%20Destroyed (+ (Variables|Default|GetFriendly%20Destroyed) 1))
        (Actor|DestroyActor (.hitactor _array_element))))))

(fn ConstructionScript)

(fn ScoreCalc1
  (bind _output_get (Variables|Default|Settemp (+ (Variables|Default|GetInherited%20Score) (Variables|Default|GetCancer%20Destroyed_R))))
  (Development|PrintString (Utilities|String|ToString(Integer) _output_get))
  (return _output_get))

(fn Score/Health)