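; HUD Blueprint that provides drag-box (marquee) selection of units.
; Marquee press, hold and release events track the drawing state and the start and current mouse positions.
; While drawing, DrawHUD renders a translucent red rectangle and queries the actors inside it every frame.
; Those actors receive a select message and join SelectedUnits, while units outside receive a deselect message and are removed during that same array's loop.
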(event EventDrawHUD
  (params (SizeX :type Integer) (SizeY :type Integer))
  (bind _startmouseposition (Variables|Default|GetStartMousePosition))
  (bind _currentmouseposition (Variables|Default|GetCurrentMousePosition))
  (if (Variables|Default|GetIsDrawing?)
    (HUD|DrawRect "(R=1.000000,G=0.000000,B=0.000000,A=0.200000)" (.x _startmouseposition) (.y _startmouseposition) (- (.x _currentmouseposition) (.x _startmouseposition)) (- (.y _currentmouseposition) (.y _startmouseposition)))
    (bind _output_get (Variables|Default|SetActorsInRectangle (Class|HUD|GetActorsinSelectionRectangle "/Script/Engine.Actor" (Variables|Default|GetStartMousePosition) (Variables|Default|GetCurrentMousePosition) false false)))
    (for _array_element _output_get
      (Class|HUDInterface|SelectUnit(Message) _array_element)
      (Utilities|Array|AddUnique (Variables|Default|GetSelectedUnits) _array_element))
    (for _array_element_2 (Variables|Default|GetSelectedUnits)
      (if (== (Utilities|Array|FindItem (Variables|Default|GetActorsInRectangle) _array_element_2) -1)
        (Class|HUDInterface|DeselectUnit(Message) _array_element_2)
        (Utilities|Array|RemoveItem (Variables|Default|GetSelectedUnits) _array_element_2)))))

(event EventMarqueePressed
  (bind _returnvalue (Game|GetPlayerController 0))
  (bind (_locationx _locationy) (Game|Player|GetMousePosition _returnvalue))
  ;[1 1 1] Marquee Start
  (Variables|Default|SetIsDrawing? true)
  (bind _output_get (Variables|Default|SetStartMousePosition (Math|Vector2D|MakeVector2D _locationx _locationy)))
  (Variables|Default|SetCurrentMousePosition _output_get))

(event EventMarqueeHeld
  (bind _returnvalue (Game|GetPlayerController 0))
  (bind (_locationx _locationy) (Game|Player|GetMousePosition _returnvalue))
  ;[1 1 1] Marquee Held
  (Variables|Default|SetCurrentMousePosition (Math|Vector2D|MakeVector2D _locationx _locationy)))

(event EventMarqueeReleased
  ;[1 1 1] Marquee Released
  (Variables|Default|SetIsDrawing? false))

(fn ConstructionScript)