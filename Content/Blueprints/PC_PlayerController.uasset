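; Player controller for a cancer-themed game, handling mouse-driven marquee selection, radiotherapy clicks, and the player's health and score.
; It shows a locked cursor and forwards left mouse press, hold (via Tick) and release to the HUD's marquee.
; When radiotherapy is prepped on BP_AbilityHandler, a click finishes it, then updates totals from destroyed counts.
; Friendly kills cost health, while cancer kills add score and restore half as much health.
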(event EventTick
  (params (DeltaSeconds :type Float%20%28single-precision%29))
  (if (Variables|Default|GetIsLeftMousePressed?)
    (Class|HUDInterface|MarqueeHeld(Message) (HUD|GetHUD))))

(event EventBeginPlay
  (Input|SetInputModeGameandUI self 0 "LockAlways" false)
  (Variables|Default|SetbShowMouseCursor true))

(event Input|MouseEvents|LeftMouseButton
  (params (Key :type Key%20Structure :default "None"))
  (:Pressed
    (bind _returnvalue (Actor|GetActorOfClass "/Game/Blueprints/BP_AbilityHandler.BP_AbilityHandler_C"))
    (bind _output_get (Variables|Default|SetAbility%20Handler%20Obj%20Ref _returnvalue))
    (if (Variables|/Game/Blueprints/BP_AbilityHandler.BP_AbilityHandler_C|GetRadioTherapyPrepped _returnvalue)
      (Default|RadioFinish _output_get)
      (bind _health (CallFunction|Score/HealthUpdate))
      (Variables|Default|SetHealth _health))))

(event Input|MouseEvents|LeftMouseButton
  (params (Key :type Key%20Structure :default "None"))
  (bind _returnvalue (HUD|GetHUD))
  (:Pressed
    (Variables|Default|SetIsLeftMousePressed? true)
    (Class|HUDInterface|MarqueePressed(Message) _returnvalue))
  (:Released
    (Variables|Default|SetIsLeftMousePressed? false)
    (Class|HUDInterface|MarqueeReleased(Message) _returnvalue)))

(fn ConstructionScript)

(fn Score/HealthUpdate
  (bind _output_get (Variables|Default|SetHealth (+ (- (Variables|Default|GetHealth) (Variables|/Game/Blueprints/BP_AbilityHandler.BP_AbilityHandler_C|GetFriendly%20Destroyed (Variables|Default|GetAbility%20Handler%20Obj%20Ref))) (Math|Float|Round (/ (Variables|/Game/Blueprints/BP_AbilityHandler.BP_AbilityHandler_C|GetCancer%20Destroyed (Variables|Default|GetAbility%20Handler%20Obj%20Ref)) 2)))))
  (bind _output_get_2 (Variables|Default|SetPCScore (+ (Variables|Default|GetPCScore) (Variables|/Game/Blueprints/BP_AbilityHandler.BP_AbilityHandler_C|GetCancer%20Destroyed (Variables|Default|GetAbility%20Handler%20Obj%20Ref)))))
  (return _output_get _output_get_2))

(fn Score/Health)