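; BP_Cell_Child_Cancer is a cancer cell variant of a parent cell Blueprint, adding a randomized spawn scatter to the parent's setup.
; On BeginPlay it nudges the flipbook up in Z, then eases the Cylinder to a random XY offset and yaw and sets an XY-plane constraint.
; After a delay it runs a second, zero-offset move, then calls MoveActor to begin movement.
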(event EventBeginPlay
  (bind _paperflipbook (Variables|Default|GetPaperFlipbook))
  (bind _cylinder (Variables|Default|GetCylinder))
  (bind _returnvalue (Transformation|GetWorldLocation _paperflipbook))
  (bind _relativelocation (Variables|/Script/Engine.SceneComponent|GetRelativeLocation _cylinder))
  (|CallParentFunction)
  (Transformation|SetWorldLocation _paperflipbook (Math|Vector|MakeVector (.x _returnvalue) (.y _returnvalue) (+ (.z _returnvalue) 0.025)) false false)
  (Components|MoveComponentTo (Variables|Default|GetCylinder) (+ _relativelocation (Math|Vector|MakeVector (Math|Random|RandomFloatinRange 8e+01 -8e+01) (Math|Random|RandomFloatinRange 8e+01 -8e+01) 0.0)) (Math|Rotator|MakeRotator 0.0 0.0 (Math|Random|RandomFloatinRange 0.0 1e+02)) false false 1.0 false)
  (Class|PrimitiveComponent|SetConstraintMode (Variables|Default|GetCylinder) "XYPlane")
  (Utilities|FlowControl|Delay 1.0)
  (Components|MoveComponentTo (Variables|Default|GetCylinder) (- _relativelocation "") "0, 0, 0" false false 1.0 false)
  (CallFunction|MoveActor))

(fn ConstructionScript
  (|CallParentFunction))