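; BP_Cell is an actor whose Cube component wanders randomly in the horizontal plane for as long as it runs.
; BeginPlay starts MoveActor, which eases the cube by a random X/Y offset from its current relative location with MoveComponentTo.
; It then sets an XY-plane constraint, waits, and runs a zero-offset move that acts as a further pause.
; MoveActor then calls itself, forming a latent loop without Tick.
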(event Custom|MoveActor
  (bind _cube (Variables|Default|GetCube))
  (bind _relativelocation (Variables|/Script/Engine.SceneComponent|GetRelativeLocation _cube))
  (Components|MoveComponentTo (Variables|Default|GetCube) (+ _relativelocation (Math|Vector|MakeVector (Math|Random|RandomFloatinRange 5e+02 -5e+02) (Math|Random|RandomFloatinRange 5e+02 -5e+02) 0.0)) "0, 0, 0" false false 1.0 false)
  (Class|PrimitiveComponent|SetConstraintMode (Variables|Default|GetCube) "XYPlane")
  (Utilities|FlowControl|Delay 1.0)
  (Components|MoveComponentTo (Variables|Default|GetCube) (- _relativelocation "0.000000,0.000000,0") "0, 0, 0" false false 1.0 false)
  (CallFunction|MoveActor))

(event EventBeginPlay
  (CallFunction|MoveActor))

(fn ConstructionScript)