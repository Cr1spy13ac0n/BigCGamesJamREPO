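; Cancer cell child Blueprint of a cell parent, which wanders randomly on its own.
; BeginPlay runs the parent logic, nudges the flipbook slightly up in Z, then sets a randomized timer to start movement.
; CancerCellMove tweens the Cylinder by a random XY offset and yaw, constrains it to the XY plane, pauses, runs a zero-offset move, then calls itself to repeat.
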(event Custom|CancerCellMove
  (bind _cylinder (Variables|Default|GetCylinder))
  (bind _relativelocation (Variables|/Script/Engine.SceneComponent|GetRelativeLocation _cylinder))
  (Components|MoveComponentTo (Variables|Default|GetCylinder) (+ _relativelocation (Math|Vector|MakeVector (Math|Random|RandomFloatinRange 1e+02 -1e+02) (Math|Random|RandomFloatinRange 1e+02 -1e+02) 0.0)) (Math|Rotator|MakeRotator 0.0 0.0 (Math|Random|RandomFloatinRange 0.0 1e+02)) false false 1.0 false)
  (Class|PrimitiveComponent|SetConstraintMode (Variables|Default|GetCylinder) "XYPlane")
  (Utilities|FlowControl|Delay 1.0)
  (Components|MoveComponentTo (Variables|Default|GetCylinder) (- _relativelocation "") "0, 0, 0" false false 1.0 false)
  (CallFunction|CancerCellMove))

(event EventBeginPlay
  (bind _paperflipbook (Variables|Default|GetPaperFlipbook))
  (bind _returnvalue (Transformation|GetWorldLocation _paperflipbook))
  (|CallParentFunction)
  (Transformation|SetWorldLocation _paperflipbook (Math|Vector|MakeVector (.x _returnvalue) (.y _returnvalue) (+ (.z _returnvalue) 0.025)) false false)
  (Utilities|Time|SetTimerbyEvent (delegate Custom|CancerCellMove) (Math|Random|RandomFloatinRange 1.5 2.0) false 0.0 1.0))

(event EventTick
  (params (DeltaSeconds :type Float%20%28single-precision%29)))

(fn ConstructionScript
  (|CallParentFunction))